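; BP_AIBase is an enemy actor, apparently the AI base, handling damage, death and boss defeat in a side-scroller.
; Any damage removes one Health, plays a hit sound and destroys the damage causer unless it is the player character.
; At zero Health it plays a flame-dependent death sound, updates player score and rank, spawns Niagara fire and destroys itself.
; Bosses also disable input, stop boss music and show the end-level widget.
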(event `DecreaseLife`
  (bind _result (`/Engine/EditorBlueprintResources/StandardMacros.DecrementInt` (`self.Health`))
    (:`  `
      (if (<= _result 0)
        (bind _asside_scroller_character (cast `/Game/SideScrollerBP/Blueprints/SideScrollerCharacter` (`GameplayStatics.GetPlayerCharacter` 0)))
        (if (`/Game/SideScrollerBP/Blueprints/SideScrollerCharacter.Can_Flame` _asside_scroller_character)
          (`AkGameplayStatics.PostEvent` "/Game/WwiseAudio/Default_Work_Unit/Play_RND_BurnEnnemi.Play_RND_BurnEnnemi")
          (else
            (`AkGameplayStatics.PostEvent` "/Game/WwiseAudio/Default_Work_Unit/Play_RND_DeathEnnemi.Play_RND_DeathEnnemi")))
        (`/Game/SideScrollerBP/Blueprints/SideScrollerCharacter.SetScore` _asside_scroller_character 0)
        (`/Game/SideScrollerBP/Blueprints/SideScrollerCharacter.CheckRank` _asside_scroller_character 200)
        (set `/Game/SideScrollerBP/Blueprints/SideScrollerCharacter.Timer_Rank` 5.0 _asside_scroller_character)
        (`NiagaraFunctionLibrary.SpawnSystemAtLocation` "/Game/Assets/VFX/BlinkAndDashVFX/VFX_Niagara/NS_Blink_Fire.NS_Blink_Fire" (`self.K2_GetActorLocation`))
        (if (`self.IsBoss`)
          (`self.DisableInput` (`GameplayStatics.GetPlayerController` 0) null)
          (`AkGameplayStatics.PostEvent` "/Game/WwiseAudio/Default_Work_Unit/Stop_BossMusic.Stop_BossMusic")
          (bind _returnvalue (`|CreateWidget` "/Game/GAme/UI/WBP_EndLevel.WBP_EndLevel_C"))
          (`UserWidget.AddToViewport` _returnvalue 0)
          (`self.K2_DestroyActor`)
          (else
            (`self.K2_DestroyActor`)))))))

(event `self.ReceiveAnyDamage`
  (params (Damage :type "Float (single-precision)") (DamageType :type "DamageType Object Reference") (InstigatedBy :type "Controller Object Reference") (DamageCauser :type "Actor Object Reference"))
  (`|ExecutionSequence`
    (:`then_0`
      (`self.DecreaseLife`)
      (`AkGameplayStatics.PostEvent` "/Game/WwiseAudio/Default_Work_Unit/Play_RND_DamageEnnemi.Play_RND_DamageEnnemi"))
    (:`then_1`
      (`/Engine/EditorBlueprintResources/StandardMacros.IsValid` DamageCauser
        (:`Is Valid`
          (cast `/Game/SideScrollerBP/Blueprints/SideScrollerCharacter` DamageCauser
            (:`CastFailed`
              (`self.K2_DestroyActor` DamageCauser))))))))

(fn `UserConstructionScript`)
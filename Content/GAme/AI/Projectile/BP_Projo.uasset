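; AI projectile that damages the side-scroller player character and penalizes its rank on hit.
; When its sphere overlaps a SideScrollerCharacter, it applies damage, resets RankScore to a fixed value chosen by the current Rank, and calls CheckRank on the character.
; It then destroys itself; overlaps with other actors are ignored, and a delay started at BeginPlay destroys it after ten seconds otherwise.
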(event `self.ReceiveBeginPlay`
  (`KismetSystemLibrary.Delay` 10.0)
  (`self.K2_DestroyActor`))

(event `self.Sphere.OnComponentBeginOverlap`
  (params (OverlappedComponent :type "PrimitiveComponent Object Reference") (OtherActor :type "Actor Object Reference") (OtherComp :type "PrimitiveComponent Object Reference") (OtherBodyIndex :type Integer) (bFromSweep :type Boolean) (SweepResult :type "HitResult Structure (by ref)"))
  (bind _asside_scroller_character (cast `/Game/SideScrollerBP/Blueprints/SideScrollerCharacter` OtherActor))
  (`GameplayStatics.ApplyDamage` _asside_scroller_character 1.0 null self)
  (switch `/Game/SideScrollerBP/Blueprints/PowerUp/E_Rank` (`/Game/SideScrollerBP/Blueprints/SideScrollerCharacter.Rank` _asside_scroller_character)
    (:`NewEnumerator3`
      (bind _output_get (set `/Game/SideScrollerBP/Blueprints/SideScrollerCharacter.RankScore` 0 _asside_scroller_character :!label _label))
      (`/Game/SideScrollerBP/Blueprints/SideScrollerCharacter.CheckRank` _asside_scroller_character _output_get))
    (:`NewEnumerator0`
      (goto _label))
    (:`NewEnumerator1`
      (bind _output_get_2 (set `/Game/SideScrollerBP/Blueprints/SideScrollerCharacter.RankScore` 500 _asside_scroller_character))
      (`/Game/SideScrollerBP/Blueprints/SideScrollerCharacter.CheckRank` _asside_scroller_character _output_get_2))
    (:`NewEnumerator2`
      (bind _output_get_3 (set `/Game/SideScrollerBP/Blueprints/SideScrollerCharacter.RankScore` 1000 _asside_scroller_character))
      (`/Game/SideScrollerBP/Blueprints/SideScrollerCharacter.CheckRank` _asside_scroller_character _output_get_3)))
  (`self.K2_DestroyActor`))

(fn `UserConstructionScript`)
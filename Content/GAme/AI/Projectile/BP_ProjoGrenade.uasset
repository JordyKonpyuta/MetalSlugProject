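; BP_ProjoGrenade is an AI grenade projectile that explodes when its mesh overlaps a SideScrollerCharacter.
; The explosion runs a sphere overlap query, spawns a Niagara effect and damages each actor found, with debug drawing and printing.
; The live path never destroys the grenade; DestroyActor sits only in a disconnected bounce-counter branch that repeats the explosion.
; Mesh hits only print the other actor.
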(event `self.StaticMesh.OnComponentBeginOverlap`
  (params (OverlappedComponent :type "PrimitiveComponent Object Reference") (OtherActor :type "Actor Object Reference") (OtherComp :type "PrimitiveComponent Object Reference") (OtherBodyIndex :type Integer) (bFromSweep :type Boolean) (SweepResult :type "HitResult Structure (by ref)"))
  (bind _returnvalue (`self.K2_GetActorLocation`))
  (cast `/Game/SideScrollerBP/Blueprints/SideScrollerCharacter` OtherActor)
  (`KismetSystemLibrary.PrintString` "GRENADE")
  (`KismetSystemLibrary.DrawDebugSphere` _returnvalue 150.0 12 (struct :`R` 1.0 :`A` 1.0) 2.0)
  (bind _outactors (`KismetSystemLibrary.SphereOverlapActors` _returnvalue 150.0 (`|MakeArray` "ObjectTypeQuery8" :!type "EObjectTypeQuery Enum") null (`|MakeArray` (`self.[ 0]`) :!type "Actor Object Reference")))
  (`self.SpawnVFX`)
  (for _array_element _outactors
    (`GameplayStatics.ApplyDamage` _array_element 1.0 null self)))

(event `self.StaticMesh.OnComponentHit`
  (params (HitComponent :type "PrimitiveComponent Object Reference") (OtherActor :type "Actor Object Reference") (OtherComp :type "PrimitiveComponent Object Reference") (NormalImpulse :type "Vector Structure") (Hit :type "HitResult Structure (by ref)"))
  (`KismetSystemLibrary.PrintString` (`KismetTextLibrary.Conv_TextToString` (`|FormatText` "Hit Grenade : {A}" OtherActor))))

(event `SpawnVFX`
  (`NiagaraFunctionLibrary.SpawnSystemAtLocation` "/Game/GAme/Niagara/Explosion/FX/NiagaraSystems/NS_Explossion.NS_Explossion" (`self.K2_GetActorLocation`)))

(fn `UserConstructionScript`)